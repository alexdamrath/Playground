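; GameModeDM is a game mode Blueprint, apparently for deathmatch, that respawns players at random spawn points.
; The Respawn event takes a controller and character and forwards them to RespawnHandler.
; RespawnHandler picks a random SpawnPoint actor in the level, spawns a new character of the same class at its transform, and has the controller possess it.
; The old character is not destroyed here.
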(event `Respawn`
  (params (PlayerController :type "Controller Object Reference") (PlayerCharacter :type "/Game/Blueprints/Ue4ASP_Character Object Reference"))
  (`self.RespawnHandler` PlayerController PlayerCharacter))

(fn `RespawnHandler`
  (params (PlayerController :type "Controller Object Reference") (PlayerCharacter :type "/Game/Blueprints/Ue4ASP_Character Object Reference"))
  (bind _outactors (`GameplayStatics.GetAllActorsOfClass` "/Game/Blueprints/SpawnPoint.SpawnPoint_C"))
  (bind _returnvalue (`|SpawnActorFromClass` (`GameplayStatics.GetObjectClass` PlayerCharacter) (`self.GetTransform` (`|GetArrayItem` _outactors (`KismetMathLibrary.RandomIntegerInRange` 0 (- (`KismetArrayLibrary.Array_Length` _outactors) 1)))) "Undefined" "OverrideRootScale" null null null))
  (`Controller.Possess` PlayerController _returnvalue))

(fn `UserConstructionScript`)