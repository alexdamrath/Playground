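; Damagable is a Blueprint that gives its owner health and handles incoming damage, apparently for networked play.
; The DamageRecieved event runs only on the server, subtracts the truncated damage value from Health and prints the new value for debugging.
; When Health drops to zero or below, it calls CallDeath.
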(event `DamageRecieved`
  (params (damageVal :type "Float (double-precision)"))
  (if (`KismetSystemLibrary.IsServer`)
    (bind _output_get (set `self.Health` (- (`self.Health`) (`KismetMathLibrary.FTrunc` damageVal))))
    (`KismetSystemLibrary.PrintString` (`KismetStringLibrary.Conv_IntToString` _output_get) true true (struct :`R` 1.0 :`B` 0.359407 :`A` 1.0))
    (if (<= _output_get 0)
      (`self.Death`))))