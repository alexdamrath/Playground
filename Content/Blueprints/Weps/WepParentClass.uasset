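; Parent weapon actor that the player can pick up and fire, with a mesh set at construction.
; Sphere overlap binds or clears the character's pickup event; pickup disables physics and collision, attaches to the first-person arms' GripPoint and switches the player's weapon.
; Player fire press and release relay through weapon dispatchers, and a tag-found FiringMode_Base component binds itself to the weapon at BeginPlay.
; OnFire only prints a debug string.
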(event `self.ReceiveBeginPlay`
  (bind _returnvalue (`self.GetComponentsByTag` "/Game/Blueprints/Weps/FiringMode_Base.FiringMode_Base_C" "PrimaryFireingMode"))
  (if (> (`KismetArrayLibrary.Array_Length` _returnvalue) 0)
    (bind _output_get (set `self.FireMode_Primary` (`|GetArrayItem` _returnvalue)))
    (`/Game/Blueprints/Weps/FiringMode_Base.SetupBinding` _output_get self)))

(event `self.Sphere.OnComponentEndOverlap`
  (params (OverlappedComponent :type "PrimitiveComponent Object Reference") (OtherActor :type "Actor Object Reference") (OtherComp :type "PrimitiveComponent Object Reference") (OtherBodyIndex :type Integer))
  (if (== (`GameplayStatics.GetObjectClass` OtherActor) "/Game/Blueprints/Ue4ASP_Character.Ue4ASP_Character_C")
    (bind _asue_4asp_character (cast `/Game/Blueprints/Ue4ASP_Character` OtherActor))
    (clear `/Game/Blueprints/Ue4ASP_Character.Pickup` _asue_4asp_character)))

(event `self.Sphere.OnComponentBeginOverlap`
  (params (OverlappedComponent :type "PrimitiveComponent Object Reference") (OtherActor :type "Actor Object Reference") (OtherComp :type "PrimitiveComponent Object Reference") (OtherBodyIndex :type Integer) (bFromSweep :type Boolean) (SweepResult :type "HitResult Structure (by ref)"))
  (if (== (`GameplayStatics.GetObjectClass` OtherActor) "/Game/Blueprints/Ue4ASP_Character.Ue4ASP_Character_C")
    (bind _asue_4asp_character (cast `/Game/Blueprints/Ue4ASP_Character` OtherActor))
    (if (!= (`/Game/Blueprints/Ue4ASP_Character.CurrentWepID` _asue_4asp_character) (`self.ID`))
      (add `/Game/Blueprints/Ue4ASP_Character.Pickup` _asue_4asp_character (delegate `OnPickup`)))))

(event `OnPickup`
  (params (Player :type "/Game/Blueprints/Ue4ASP_Character Object Reference"))
  (bind _box (`self.Box`))
  (add `/Game/Blueprints/Ue4ASP_Character.PrimaryFire` Player (delegate `PrimaryCallback`))
  (add `/Game/Blueprints/Ue4ASP_Character.PrimaryUp` Player (delegate `PrimaryUpCallback`))
  (set `self.OwnerRef` Player)
  (`PrimitiveComponent.SetEnableGravity` _box false)
  (`PrimitiveComponent.SetSimulatePhysics` _box false)
  (`PrimitiveComponent.SetCollisionEnabled` _box "NoCollision")
  (`PrimitiveComponent.SetCollisionEnabled` (`self.Sphere`) "NoCollision")
  (`self.SetOwner` Player)
  (`self.K2_AttachToComponent` (`/Game/Blueprints/Ue4ASP_Character.FP_Arms` Player) "GripPoint" "SnapToTarget" "SnapToTarget" "KeepRelative")
  (set `self.PickedUp` true)
  (`/Game/Blueprints/Ue4ASP_Character.SwitchWeapons` Player (`self.NewWepMesh`) (`self.ID`))
  (`PrimitiveComponent.SetOnlyOwnerSee` (`self.Wep Mesh`) true)
  (clear `/Game/Blueprints/Ue4ASP_Character.Pickup` Player))

(event `PrimaryCallback`
  (`self.PrimaryDown`))

(event `PrimaryUpCallback`
  (`self.PrimaryUp`))

(event `OnFire`
  (`KismetSystemLibrary.PrintString` "parent class fired"))

(fn `UserConstructionScript`
  (`StaticMeshComponent.SetStaticMesh` (`self.Wep Mesh`) (`self.NewWepMesh`)))