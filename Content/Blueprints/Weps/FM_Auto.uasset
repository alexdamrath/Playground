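; FM_Auto is an automatic fire mode for weapons that fires repeatedly from BeginFire until EndFire.
; BeginFire opens a Gate and enters it at once, so the first shot is immediate.
; Each pass calls Fire, then waits FireRate in a Delay before re-entering the Gate, forming a loop without Tick.
; EndFire closes the Gate, which stops the loop at its next pass.
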(event `self.BeginFire`
  (`|ExecutionSequence`
    (:`then_0`
      (goto _label :!via `Open`))
    (:`then_1`
      (`/Engine/EditorBlueprintResources/StandardMacros.Gate` true :!label _label
        (:`Exit`
          (`|ExecutionSequence`
            (:`then_0`
              (`self.Fire`))
            (:`then_1`
              (`KismetSystemLibrary.Delay` (`self.FireRate`))
              (goto _label))))))))

(event `self.EndFire`
  (goto _label :!via `Close`))