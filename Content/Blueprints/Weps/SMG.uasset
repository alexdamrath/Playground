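; SMG weapon Blueprint that fires automatic hitscan shots from the player camera.
; On BeginPlay it binds PrimaryFire to the FMAuto fire-mode component and passes it the rate of fire.
; Each shot runs a debug-drawn Visibility line trace that ignores the owner and damages only actors with a Damagable component.
; Hits on components tagged "head" deal double damage, credited to the owner's controller.
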(event `self.ReceiveBeginPlay`
  (bind _fm_auto (`self.FM_Auto`))
  (`parent.ReceiveBeginPlay`)
  (add `/Game/Blueprints/Weps/FiringMode_Base.Fire` _fm_auto (delegate `Primary Fire`))
  (set `/Game/Blueprints/Weps/FiringMode_Base.FireRate` (`self.RateOfFire`) _fm_auto))

(event `Primary Fire`
  (bind _returnvalue (`GameplayStatics.GetPlayerCameraManager` 0))
  (bind _damage (`self.Damage`))
  (bind _returnvalue_2 (`self.K2_GetActorLocation` _returnvalue))
  (bind _returnvalue_3 (`self.GetActorForwardVector` _returnvalue))
  (bind (_outhit _returnvalue_4) (`KismetSystemLibrary.LineTraceSingle` (+ (* _returnvalue_3 50.0) _returnvalue_2) (+ (* _returnvalue_3 5000.0) _returnvalue_2) "TraceTypeQuery1" false (`|MakeArray` (`self.OwnerRef`)) "ForDuration" true (struct :`R` 1.0 :`A` 1.0) (struct :`G` 1.0 :`A` 1.0) 2.0))
  (if _returnvalue_4
    (bind (_bblockinghit _binitialoverlap _time _distance _location _impactpoint _normal _impactnormal _physmat _hitactor _hitcomponent) (`GameplayStatics.BreakHitResult` _outhit))
    (`/Engine/EditorBlueprintResources/StandardMacros.IsValid` (`self.GetComponentByClass` _hitactor "/Game/Blueprints/Damagable.Damagable_C")
      (:`Is Valid`
        (`GameplayStatics.ApplyDamage` _hitactor (select `bool` (`ActorComponent.ComponentHasTag` _hitcomponent "head") :`false` _damage :`true` (* _damage 2.0)) (`Pawn.GetController` (`self.OwnerRef`)) self)))))

(fn `UserConstructionScript`
  (`parent.UserConstructionScript`))